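; BP_Crystal is a crystal actor that is resized and rotated through four slider controls.
; Each slider's value-updated event writes straight to the actor transform, with the resize value used as a uniform scale.
; The three rotation sliders scale their value by a constant into roll, pitch or yaw.
; Each sets an absolute rotation with only its own axis supplied, so the axes do not combine.
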(event `self.Slider_Resize.OnValueUpdated`
  (params (Slider :type "UxtPinchSliderActor Object Reference") (NewValue :type "Float (single-precision)"))
  (bind _returnvalue (* (`UxtPinchSliderActor.Value` (`self.Slider_Resize`)) 1.0))
  (`self.SetActorScale3D` (`KismetMathLibrary.MakeVector` _returnvalue _returnvalue _returnvalue)))

(event `self.Slider_RotatorX.OnValueUpdated`
  (params (Slider :type "UxtPinchSliderActor Object Reference") (NewValue :type "Float (single-precision)"))
  (`self.K2_SetActorRotation` (`KismetMathLibrary.MakeRotator` (* (`UxtPinchSliderActor.Value` (`self.Slider_RotatorX`)) 100.0))))

(event `self.Slider_RotateY.OnValueUpdated`
  (params (Slider :type "UxtPinchSliderActor Object Reference") (NewValue :type "Float (single-precision)"))
  (`self.K2_SetActorRotation` (`KismetMathLibrary.MakeRotator` 0.0 (* (`UxtPinchSliderActor.Value` (`self.Slider_RotateY`)) 100.0))))

(event `self.Slider_RotateZ.OnValueUpdated`
  (params (Slider :type "UxtPinchSliderActor Object Reference") (NewValue :type "Float (single-precision)"))
  (`self.K2_SetActorRotation` (`KismetMathLibrary.MakeRotator` 0.0 0.0 (* (`UxtPinchSliderActor.Value` (`self.Slider_RotateZ`)) 100.0))))

(fn `UserConstructionScript`)