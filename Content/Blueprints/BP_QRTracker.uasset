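; QR code tracker Blueprint for AR that listens to tracked-geometry updates through an ARTrackableNotify component.
; Each update that casts to ARTrackedQRCode prints the code's unique ID; the add event does nothing.
; Disconnected, never-run branches hold string matches for "Vodka" and "Nokia" that would each spawn an animation actor once, guarded by booleans.
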(event `self.ARTrackableNotify.OnAddTrackedGeometry`
  (params (TrackedGeometry :type "ARTrackedGeometry Object Reference")))

(event `self.ARTrackableNotify.OnUpdateTrackedGeometry`
  (params (TrackedGeometry :type "ARTrackedGeometry Object Reference"))
  (bind _asartracked_qrcode (cast `ARTrackedQRCode` TrackedGeometry))
  (`KismetSystemLibrary.PrintString` (`KismetGuidLibrary.Conv_GuidToString` (`ARTrackedGeometry.UniqueId` _asartracked_qrcode))))

(fn `UserConstructionScript`)