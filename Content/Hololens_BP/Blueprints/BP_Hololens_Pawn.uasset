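; HoloLens player pawn for a collaborative AR app, running the AR session and driving hand-tracked interaction and avatar head.
; Fingertip presses pick actors and fire the contextual menu's current option; grabbed actors follow interpolation-smoothed wrist transforms while the transform component ticks.
; Wrist-attached buttons open a camera-placed menu that auto-hides on a retriggerable delay, with widget interaction at the fingertips.
; The locally controlled pawn sends its head pose through a server-update event.
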(event `self.ReceiveTick`
  (params (DeltaSeconds :type "Float (single-precision)"))
  ;[0.7995 0.05269 0] Tick
  (`|ExecutionSequence`
    (:`then_0`
      (`|ExecutionSequence`
        (:`then_0`
          (`self.SetControllerWorldTansform` true)
          (`self.SmoothedTransforms` true)
          (`self.MoveActor` true))
        (:`then_1`
          (`self.SetControllerWorldTansform` false)
          (`self.SmoothedTransforms` false)
          (`self.MoveActor` false))))
    (:`then_1`
      (`self.FingerDebugLocation`)
      (`self.ContextualMenuFollowWrist`)
      (`self.InterationIndex`))
    (:`then_2`
      (`self.UpdateHeadOnServer`)
      (`self.UpdateAvatarPosition`))))

(event `Destroyed` :!signature `self.OnDestroyed`
  (params (DestroyedActor :type "Actor Object Reference"))
  ;[0.01836 1 0] Bring Back The Menu on desktop after destroyed Pawn
  (`ARBlueprintLibrary.StopARSession`)
  (bind _asbp_collab_v_player_controller (cast `/Game/CollaborativeViewer/Blueprints/PlayerController/BP_Collab_V_PlayerController` (`GameplayStatics.GetPlayerController` 0)))
  (bind _desktop_ui (`/Game/CollaborativeViewer/Blueprints/PlayerController/BP_Collab_V_PlayerController.Desktop_UI` _asbp_collab_v_player_controller))
  (if (not (`Widget.IsInViewport` _desktop_ui))
    (`UserWidget.AddToViewport` _desktop_ui 0)
    (`UserWidget.AddToViewport` (`/Game/CollaborativeViewer/Blueprints/PlayerController/BP_Collab_V_PlayerController.Persistent_UI` _asbp_collab_v_player_controller) 0)))

(event `self.ReceivePossessed`
  (params (NewController :type "Controller Object Reference"))
  ;[0.1183 1 0] Begin Play
  (`self.PossesedARPawn` NewController))

(event `self.ReceiveBeginPlay`
  (set `self.NavigationMode` "NewEnumerator2")
  (set `/Game/CollaborativeViewer/Blueprints/Commands/Annotation/BP_AnnotationComponent.EnableTextCommand` false (`self.AnnotationComponent`))
  (set `self.ExecuteMenuUnhovered` true)
  ;[0.1183 1 0] Begin Play
  (set `self.SpawnLaser` false)
  (set `self.IsVR` true)
  (`parent.ReceiveBeginPlay`)
  (`|ExecutionSequence`
    (:`then_0`
      ;[0.01836 1 0] Start AR Session
      (`ARBlueprintLibrary.StartARSession` "/Game/Hololens_BP/Blueprints/ARSessionConfig.ARSessionConfig"))
    (:`then_1`
      ;[0.01836 1 0] Bring Back The Menu on desktop after destroyed Pawn
      (add `self.OnDestroyed` (delegate `Destroyed`)))
    (:`then_2`
      ;[0.01836 1 0] Hand Bindings On pressed and Released fingers
      (`self.BindRightHand`)
      (`self.BindLeftHand`))
    (:`then_3`
      ;[0.01836 1 0] Set up Avatar Color
      (`KismetArrayLibrary.Array_Append` (`self.PlayerMeshesArray`) (`|MakeArray` (`self.VR_Mesh`) null (`self.BaseRing`) (`self.BaseRing_Glow`) (`self.Head_Mesh`) null null null :!type "PrimitiveComponent Object Reference")))
    (:`then_4`
      ;[0.01836 1 0] Set up Anotation Component
      (add `WidgetInteractionComponent.OnHoveredWidgetChanged` (`self.WidgetInteractionR`) (delegate `RetriggerMenuOnHovered`))
      (add `WidgetInteractionComponent.OnHoveredWidgetChanged` (`self.WidgetInteractionL`) (delegate `RetriggerMenuOnHovered`)))
    (:`then_5`
      (`ActorComponent.SetComponentTickEnabled` (`self.TransformComponent`) false)
      (set `/Game/CollaborativeViewer/Blueprints/Commands/Transform/BP_TransformComponent.IsActivated` false (`self.TransformComponent`)))))

(event `self.ContextualWidgetDone`
  (bind _contextualwidget (`self.ContextualWidget`))
  ;[0.01836 1 0] SetWidgets
  (`WidgetComponent.SetWidget` (`self.ContextualWidget_VR`) (`self.ContextualWidget`))
  (`WidgetComponent.SetWidget` (`self.Current_Widget_VR`) (`/Game/CollaborativeViewer/UMG/GameMenu/Destop_UI.Current_Command_Widget` (`/Game/CollaborativeViewer/Blueprints/PlayerController/BP_Collab_V_PlayerController.Desktop_UI` (cast `/Game/CollaborativeViewer/Blueprints/PlayerController/BP_Collab_V_PlayerController` (`GameplayStatics.GetPlayerController` 0) :!pure true))))
  (if (`Widget.IsInViewport` _contextualwidget)
    (`Widget.RemoveFromParent` _contextualwidget)))

(event `RetriggerMenuOnHovered`
  (params (WidgetComponent :type "WidgetComponent Object Reference") (PreviousWidgetComponent :type "WidgetComponent Object Reference"))
  ;[0.01836 1 0] Set up Anotation Component
  (`self.Retrigger_HideMenu`))

(event `PossesedARPawn`
  (params (Controller :type "Controller Object Reference"))
  ;[0.2555 0.7775 1] ON_Possessed
  (`/Engine/EditorBlueprintResources/StandardMacros.IsValid` Controller
    (:`Is Valid`
      (if (`Controller.IsLocalPlayerController` Controller)
        _))))

(event `BindLeftHand`
  (bind _leftfingertipbutton (`self.LeftFingerTipButton`))
  ;[0.2555 0.7775 1] Fingers Tip  Pressed Binding
  (add `/Game/Hololens_BP/Blueprints/BP_GraspedAction.TipPressed` _leftfingertipbutton (`|CreateDelegate` :!event `BindLeftHandPressed`))
  (add `/Game/Hololens_BP/Blueprints/BP_GraspedAction.TipReleased` _leftfingertipbutton (`|CreateDelegate` :!event `BindLeftHandREleased`)))

(event `BindRightHand`
  (bind _rightfingertipbutton (`self.RightFingerTipButton`))
  ;[0.2555 0.7775 1] Fingers Tip  Pressed Binding
  (add `/Game/Hololens_BP/Blueprints/BP_GraspedAction.TipPressed` _rightfingertipbutton (`|CreateDelegate` :!event `BindRightHandPressed`))
  (add `/Game/Hololens_BP/Blueprints/BP_GraspedAction.TipReleased` _rightfingertipbutton (`|CreateDelegate` :!event `BindRightHandReleased`)))

(event `self.MenuButtonL.OnComponentBeginOverlap`
  (params (OverlappedComponent :type "PrimitiveComponent Object Reference") (OtherActor :type "Actor Object Reference") (OtherComp :type "PrimitiveComponent Object Reference") (OtherBodyIndex :type Integer) (bFromSweep :type Boolean) (SweepResult :type "HitResult Structure (by ref)"))
  ;[0.2555 0.7775 1] Show Contextual Menu On component Overlap
  (`self.MenuShow` :!label _label))

(event `UpdateAvatarPosition`
  (bind (_returnvalue_x _returnvalue_y _returnvalue_z) (`KismetMathLibrary.BreakVector` (`self.K2_GetActorLocation`)))
  (bind (_headpos_x _headpos_y) (`KismetMathLibrary.BreakVector` (`self.HeadPos`)))
  ;[0.2555 0.7775 1] Update avatar position
  (`SceneComponent.K2_SetWorldLocation` (`self.BaseRing_Glow`) (`KismetMathLibrary.MakeVector` _headpos_x _headpos_y _returnvalue_z) false false))

(event `ContextualMenuFollowWrist`
  ;[0.2555 0.7775 1] Menu Trigger Follow Wrist
  (`|ExecutionSequence`
    (:`then_0`
      (bind _transform (`/Game/Hololens_BP/Blueprints/BP_GraspedAction.GetHandJointTransform` (`self.LeftFingerTipButton`) "Left" 0 (`self.leftWristTransform`)))
      (bind _output_get (set `self.leftWristTransform` _transform))
      (`SceneComponent.K2_SetWorldTransform` (`self.RootMenuButtonL`) (`KismetMathLibrary.MakeTransform` (.location _output_get) (.rotation _output_get) (`KismetMathLibrary.Conv_DoubleToVector` 0.07)) false false))
    (:`then_1`
      (bind _transform_2 (`/Game/Hololens_BP/Blueprints/BP_GraspedAction.GetHandJointTransform` (`self.RightFingerTipButton`) "Right" 0 (`self.rightWristTransform`)))
      (bind _output_get_2 (set `self.rightWristTransform` _transform_2))
      (`SceneComponent.K2_SetWorldTransform` (`self.RootMenuButtonR`) (`KismetMathLibrary.MakeTransform` (.location _output_get_2) (.rotation _output_get_2) (`KismetMathLibrary.Conv_DoubleToVector` 0.07)) false false))))

(event `self.MenuButtonR.OnComponentBeginOverlap`
  (params (OverlappedComponent :type "PrimitiveComponent Object Reference") (OtherActor :type "Actor Object Reference") (OtherComp :type "PrimitiveComponent Object Reference") (OtherBodyIndex :type Integer) (bFromSweep :type Boolean) (SweepResult :type "HitResult Structure (by ref)"))
  ;[0.2555 0.7775 1] Show Contextual Menu On component Overlap
  (goto _label))

(event `BindLeftHandPressed`
  ;[0.2555 0.7775 1] Fingers Tip  Pressed Binding
  (set `self.LeftHandPressed` true)
  (`self.SetControllerWorldTansform` false true)
  (bind _validhit (`self.SetPickedActor` false (`self.CollisionType`)))
  (set `self.Left_Grabbed` _validhit)
  (bind _currentoption (`/Game/CollaborativeViewer/UMG/GameMenu/Contextual_Widget.CurrentOption` (`self.ContextualWidget`))
    (:`then`
      (`/Game/CollaborativeViewer/UMG/GameMenu/Option_Button.DoIt` _currentoption (`self.CurrentHitActor_L`) false))
    (:`else`)))

(event `BindRightHandPressed`
  ;[0.2555 0.7775 1] Fingers Tip  Pressed Binding
  (set `self.RightHandPressed` true)
  (`self.SetControllerWorldTansform` true true)
  (bind _validhit (`self.SetPickedActor` true (`self.CollisionType`)))
  (set `self.Right_Grabbed` _validhit)
  (bind _currentoption (`/Game/CollaborativeViewer/UMG/GameMenu/Contextual_Widget.CurrentOption` (`self.ContextualWidget`))
    (:`then`
      (`/Game/CollaborativeViewer/UMG/GameMenu/Option_Button.DoIt` _currentoption (`self.CurrentHitActor_R`) true))
    (:`else`)))

(event `EventUpdateCameraToServer`
  (params (HeadPosition :type "Vector Structure") (HeadRotation :type "Rotator Structure"))
  ;[0.2555 0.7775 1] updateHand
  (set `self.HeadPos` HeadPosition)
  (set `self.HeadRot` HeadRotation))

(event `SetContextualMenuLocation`
  (bind _returnvalue (`SceneComponent.K2_GetComponentToWorld` (`self.Camera`)))
  ;[0.2555 0.7775 1] ContextualMenuLocation
  (`SceneComponent.K2_SetWorldTransform` (`self.RootMenu`) (`KismetMathLibrary.MakeTransform` (.location _returnvalue) (`KismetMathLibrary.MakeRotator` 0.0 (.pitch (.rotation _returnvalue)) (.yaw (.rotation _returnvalue))) (`KismetMathLibrary.Conv_DoubleToVector` 0.7)) false false))

(event `BindLeftHandReleased`
  ;[0.2555 0.7775 1] Fingers Tip  Pressed Binding
  (set `self.LeftHandPressed` false)
  (`self.setCustomDepth_runOnServer` (`self.CurrentHitActor_L`))
  (set `self.CurrentHitActor_L` null)
  (set `self.Left_Grabbed` false)
  (bind _currentoption (`/Game/CollaborativeViewer/UMG/GameMenu/Contextual_Widget.CurrentOption` (`self.ContextualWidget`))
    (:`then`
      (`/Game/CollaborativeViewer/UMG/GameMenu/Option_Button.DoItOnReleased` _currentoption null false false))
    (:`else`)))

(event `UpdateHeadOnServer`
  (bind _camera (`self.Camera`))
  ;[0.2555 0.7775 1] updateHand
  (if (`self.IsLocallyControlled`)
    (set `self.HeadPos` (`SceneComponent.K2_GetComponentLocation` _camera))
    (set `self.HeadRot` (`SceneComponent.K2_GetComponentRotation` _camera))
    (`self.EventUpdateCameraToServer` (`self.HeadPos`) (`self.HeadRot`)))
  (`SceneComponent.K2_SetWorldLocationAndRotation` (`self.Head_Mesh`) (`self.HeadPos`) (`KismetMathLibrary.MakeRotator` (* (.pitch (`KismetMathLibrary.ComposeRotators` (`self.HeadRot`) (struct :`Yaw` -90.0))) -1.0) (.roll (`KismetMathLibrary.ComposeRotators` (`self.HeadRot`) (struct :`Yaw` -90.0))) (.yaw (`KismetMathLibrary.ComposeRotators` (`self.HeadRot`) (struct :`Yaw` -90.0)))) false false))

(event `BindRightHandReleased`
  ;[0.2555 0.7775 1] Fingers Tip  Pressed Binding
  (set `self.RightHandPressed` false)
  (`self.setCustomDepth_runOnServer` (`self.CurrentHitActor_R`))
  (set `self.CurrentHitActor_R` null)
  (set `self.Right_Grabbed` false)
  (bind _currentoption (`/Game/CollaborativeViewer/UMG/GameMenu/Contextual_Widget.CurrentOption` (`self.ContextualWidget`))
    (:`then`
      (`/Game/CollaborativeViewer/UMG/GameMenu/Option_Button.DoItOnReleased` _currentoption null true false))
    (:`else`)))

(event `MenuShow`
  (bind _contextualwidget (`self.ContextualWidget`))
  ;[0.2555 0.7775 1] MenuVIsibility
  (`|ExecutionSequence`
    (:`then_0`
      (`self.SetContextualMenuLocation`)
      (if (not (`self.isContextualMenu`))
        (`/Engine/EditorBlueprintResources/StandardMacros.IsValid` _contextualwidget
          (:`Is Valid`
            (`/Game/CollaborativeViewer/UMG/GameMenu/Contextual_Widget.ShowHideContextualMenu` _contextualwidget "Visible")
            (set `self.isContextualMenu` true)))))
    (:`then_1`
      (`self.Retrigger_HideMenu`))))

(event `InterationIndex`
  (bind (_fingertip_transform_location _fingertip_transform_rotation) (`KismetMathLibrary.BreakTransform` (`/Game/Hololens_BP/Blueprints/BP_GraspedAction.FingerTip_Transform` (`self.LeftFingerTipButton`))))
  (bind (_fingertip_transform_location_2 _fingertip_transform_rotation_2) (`KismetMathLibrary.BreakTransform` (`/Game/Hololens_BP/Blueprints/BP_GraspedAction.FingerTip_Transform` (`self.RightFingerTipButton`))))
  ;[0.2555 0.7775 1] Set Widget Interaction to the index Location
  (`SceneComponent.K2_SetWorldLocationAndRotation` (`self.InteractionRootR`) _fingertip_transform_location_2 _fingertip_transform_rotation_2 false false)
  (`SceneComponent.K2_SetWorldLocationAndRotation` (`self.InteractionRootL`) _fingertip_transform_location _fingertip_transform_rotation false false))

(event `Retrigger_HideMenu`
  ;[0.2555 0.7775 1] MenuVIsibility
  (`KismetSystemLibrary.RetriggerableDelay` 3.0)
  (`/Game/CollaborativeViewer/UMG/GameMenu/Contextual_Widget.ShowHideContextualMenu` (`self.ContextualWidget`) "Collapsed")
  (set `self.isContextualMenu` false))

(event `SetControllerWorldTansform`
  (params (IsRight :type Boolean) (FirstSetup :type Boolean :default false))
  (bind _rightfingertipbutton (`self.RightFingerTipButton`))
  (bind _leftfingertipbutton (`self.LeftFingerTipButton`))
  (bind (_middletransform_location _middletransform_rotation) (`KismetMathLibrary.BreakTransform` (`/Game/Hololens_BP/Blueprints/BP_GraspedAction.MiddleTransform` _rightfingertipbutton)))
  (bind (_wristtransform_location _wristtransform_rotation) (`KismetMathLibrary.BreakTransform` (`/Game/Hololens_BP/Blueprints/BP_GraspedAction.WristTransform` _rightfingertipbutton)))
  (bind (_middletransform_location_2 _middletransform_rotation_2) (`KismetMathLibrary.BreakTransform` (`/Game/Hololens_BP/Blueprints/BP_GraspedAction.MiddleTransform` _leftfingertipbutton)))
  (bind (_wristtransform_location_2 _wristtransform_rotation_2) (`KismetMathLibrary.BreakTransform` (`/Game/Hololens_BP/Blueprints/BP_GraspedAction.WristTransform` _leftfingertipbutton)))
  ;[0.2555 0.7775 1] Set Finger Tip World Tansform
  (if IsRight
    (bind _output_get (set `self.TipFingerControllerTransform_R` (`KismetMathLibrary.MakeTransform` _middletransform_location _middletransform_rotation)))
    (bind _output_get_2 (set `self.WristControllerTransform_R` (`KismetMathLibrary.MakeTransform` _wristtransform_location _wristtransform_rotation)))
    (if FirstSetup
      (bind _output_get_3 (set `self.FingerTransformSmoothed_R` _output_get))
      (set `self.TransformControllerR` _output_get_3)
      (set `self.WristTransformSmoothed_R` _output_get_2))
    (else
      (bind _output_get_4 (set `self.TipFingerControllerTransform_L` (`KismetMathLibrary.MakeTransform` _middletransform_location_2 _middletransform_rotation_2)))
      (bind _output_get_5 (set `self.WristControllerTransform_L` (`KismetMathLibrary.MakeTransform` _wristtransform_location_2 _wristtransform_rotation_2)))
      (if FirstSetup
        (bind _output_get_6 (set `self.FingerTransformSmoothed_L` _output_get_4))
        (set `self.TransformControllerL` _output_get_6)
        (set `self.WristTransformSmoothed_L` _output_get_5)))))

(event `FingerDebugLocation`
  (bind _fingertip_transform_location (`KismetMathLibrary.BreakTransform` (`/Game/Hololens_BP/Blueprints/BP_GraspedAction.FingerTip_Transform` (`self.LeftFingerTipButton`))))
  (bind _fingertip_transform_location_2 (`KismetMathLibrary.BreakTransform` (`/Game/Hololens_BP/Blueprints/BP_GraspedAction.FingerTip_Transform` (`self.RightFingerTipButton`))))
  ;[0.2555 0.7775 1] Finger Debug meshes Location
  (`SceneComponent.K2_SetWorldLocation` (`self.RightHandFinger`) _fingertip_transform_location_2 false false)
  (`SceneComponent.K2_SetWorldLocation` (`self.LeftHandFinger`) _fingertip_transform_location false false))

(event `JoinSessionWithIP`
  ;[1 1 1] Manually join a session
  (`KismetSystemLibrary.ExecuteConsoleCommand` (`KismetStringLibrary.Concat_StrStr` "open " (`KismetTextLibrary.Conv_TextToString` (`EditableTextBox.GetText` (`self.IP_Address`)))) (`GameplayStatics.GetPlayerController` 0)))

(event `MoveActor`
  (params (IsRightHand :type Boolean))
  (bind _currenthitactor_r (`self.CurrentHitActor_R`))
  (bind _currenthitactor_l (`self.CurrentHitActor_L`))
  (bind (_returnvalue_location _returnvalue_rotation _returnvalue_scale) (`KismetMathLibrary.BreakTransform` (`KismetMathLibrary.ComposeTransforms` (`self.RelativeStartTransform_R`) (`self.WristTransformSmoothed_R`))))
  (bind (_returnvalue_location_2 _returnvalue_rotation_2 _returnvalue_scale_2) (`KismetMathLibrary.BreakTransform` (`KismetMathLibrary.ComposeTransforms` (`self.RelativeStartTransform_L`) (`self.WristTransformSmoothed_L`))))
  ;[0.2555 0.7775 1] Move Actor
  (if IsRightHand
    (if (and (`self.Right_Grabbed`) (`ActorComponent.IsComponentTickEnabled` (`self.TransformComponent`)))
      (`/Engine/EditorBlueprintResources/StandardMacros.IsValid` _currenthitactor_r
        (:`Is Valid`
          (set `/Game/CollaborativeViewer/Blueprints/Commands/Transform/BP_TransformComponent.FinalTransformR` (`KismetMathLibrary.MakeTransform` _returnvalue_location _returnvalue_rotation _returnvalue_scale) (`self.TransformComponent`))
          (`self.K2_SetActorTransform` _currenthitactor_r (`KismetMathLibrary.MakeTransform` _returnvalue_location _returnvalue_rotation _returnvalue_scale) false false))))
    (elif (and (`self.Left_Grabbed`) (`ActorComponent.IsComponentTickEnabled` (`self.TransformComponent`)))
      (`/Engine/EditorBlueprintResources/StandardMacros.IsValid` _currenthitactor_l
        (:`Is Valid`
          (set `/Game/CollaborativeViewer/Blueprints/Commands/Transform/BP_TransformComponent.FinalTransformL` (`KismetMathLibrary.MakeTransform` _returnvalue_location_2 _returnvalue_rotation_2 _returnvalue_scale_2) (`self.TransformComponent`))
          (`self.K2_SetActorTransform` _currenthitactor_l (`KismetMathLibrary.MakeTransform` _returnvalue_location_2 _returnvalue_rotation_2 _returnvalue_scale_2) false false))))))

(event `CreateSession`
  (`CreateSessionCallbackProxy.CreateSession` (`GameplayStatics.GetPlayerController` 0) 10
    (:`OnSuccess`
      (`GameplayStatics.OpenLevel` "ArLevel" true "listen"))))

(event `SmoothedTransforms`
  (params (IsRightHand :type Boolean :default true))
  ;[0.2555 0.7775 1] Smoothing Transforms
  (if IsRightHand
    (set `self.WristTransformSmoothed_R` (`KismetMathLibrary.TInterpTo` (`self.WristTransformSmoothed_R`) (`self.WristControllerTransform_R`) (`GameplayStatics.GetWorldDeltaSeconds`) 20.0))
    (bind _output_get (set `self.FingerTransformSmoothed_R` (`KismetMathLibrary.TInterpTo` (`self.FingerTransformSmoothed_R`) (`self.TipFingerControllerTransform_R`) (`GameplayStatics.GetWorldDeltaSeconds`) 20.0)))
    (set `self.TransformControllerR` _output_get)
    (else
      (set `self.WristTransformSmoothed_L` (`KismetMathLibrary.TInterpTo` (`self.WristTransformSmoothed_L`) (`self.WristControllerTransform_L`) (`GameplayStatics.GetWorldDeltaSeconds`) 20.0))
      (bind _output_get_2 (set `self.FingerTransformSmoothed_L` (`KismetMathLibrary.TInterpTo` (`self.FingerTransformSmoothed_L`) (`self.WristControllerTransform_L`) (`GameplayStatics.GetWorldDeltaSeconds`) 20.0)))
      (set `self.TransformControllerL` _output_get_2))))

(fn `SetPickedActor`
  (params (IsRight :type Boolean) (ObjectTypes :type "Array of EObjectTypeQuery Enum (by ref)"))
  (returns (ValidHit :type Boolean))
  (locals (IsValidHit_Local :type Boolean :default true) (IsRight_Local :type Boolean))
  (bind _returnvalue (select `bool` (`local.IsRight_Local`) :`false` (`self.LeftFingerTipButton`) :`true` (`self.RightFingerTipButton`)))
  (bind _hitactor (`/Game/Hololens_BP/Blueprints/BP_GraspedAction.HitActor` _returnvalue))
  (bind _returnvalue_2 (`KismetMathLibrary.MakeRelativeTransform` (`self.GetTransform` (select `bool` (`local.IsRight_Local`) :`false` (`self.CurrentHitActor_L`) :`true` (`self.CurrentHitActor_R`))) (select `bool` (`local.IsRight_Local`) :`false` (`self.WristControllerTransform_L`) :`true` (`self.WristControllerTransform_R`))))
  (set `local.IsRight_Local` IsRight)
  (bind _hitvalid (`/Game/Hololens_BP/Blueprints/BP_GraspedAction.GetHitOnFingerTip` _returnvalue ObjectTypes))
  (if _hitvalid
    (if (`local.IsRight_Local`)
      (set `self.CurrentHitActor_R` _hitactor)
      (else
        (set `self.CurrentHitActor_L` _hitactor)))
    (`/Engine/EditorBlueprintResources/StandardMacros.IsValid` _hitactor
      (:`Is Valid`
        (set `local.IsValidHit_Local` true)
        (if (`local.IsRight_Local`)
          (set `self.RelativeStartTransform_R` _returnvalue_2)
          (else
            (set `self.RelativeStartTransform_L` _returnvalue_2))))
      (:`Is Not Valid`
        (set `local.IsValidHit_Local` false)))
    (return (`local.IsValidHit_Local`))
    (else
      (set `self.CurrentHitActor_R` null)
      (set `self.CurrentHitActor_L` null))))

(fn `UserConstructionScript`
  (`parent.UserConstructionScript`))